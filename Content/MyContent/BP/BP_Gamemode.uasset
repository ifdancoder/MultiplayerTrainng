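; BP_Gamemode is a game mode that balances joining players between two teams.
; PostLogin casts each new player to BP_MultiplayerController, sets its team ID to the team with fewer members (team 1 on a tie) and increments that count, printing an error if the cast fails.
; OnLogout only casts the exiting controller, so team counts are never decremented when players leave.
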(event EventBeginPlay)

(event EventTick
  (params (DeltaSeconds :type Float%20%28single-precision%29)))

(event EventPostLogin
  (params (NewPlayer :type Player%20Controller%20Object%20Reference))
  (bind _asbp_multiplayer_controller (Utilities|Casting|CastToBP_MultiplayerController NewPlayer)
    (:then
      (if (< (Variables|Default|GetTeam2Num) (Variables|Default|GetTeam1Num))
        (Default|SetTeamID _asbp_multiplayer_controller 2)
        (Variables|Default|SetTeam2Num (+ (Variables|Default|GetTeam2Num) 1))
        (else
          (Default|SetTeamID _asbp_multiplayer_controller 1)
          (Variables|Default|SetTeam1Num (+ (Variables|Default|GetTeam1Num) 1)))))
    (:CastFailed
      (Development|PrintString "Post login error"))))

(event EventOnLogout
  (params (ExitingController :type Controller%20Object%20Reference))
  (Utilities|Casting|CastToBP_MultiplayerController ExitingController))

(fn ConstructionScript)