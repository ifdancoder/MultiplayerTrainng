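; Networked projectile that flies forward and damages the BP_MultiplayerPlayerPawn it overlaps.
; The server moves it each tick by Speed without sweeping and handles sphere overlaps, ignoring the owner and other projectiles.
; Any other hit triggers a multicast explosion effect and destroys the projectile, with damage applied only to player pawns.
; A TTL timer started on BeginPlay also destroys it through the server end-of-life event.
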(event OnComponentBeginOverlap(Sphere1)
  (params (OverlappedComponent :type Primitive%20Component%20Object%20Reference) (OtherActor :type Actor%20Object%20Reference) (OtherComp :type Primitive%20Component%20Object%20Reference) (OtherBodyIndex :type Integer) (bFromSweep :type Boolean) (SweepResult :type Hit%20Result%20Structure%20%28by%20ref%29))
  (if (Networking|IsServer)
    (CallFunction|ServerCollision OtherActor (Transformation|GetActorLocation))))

(event Custom|server_collision
  (params (Other%20Actor :type Actor%20Object%20Reference) (Location :type Vector))
  (if (!= Other%20Actor (Components|GetOwner))
    (bind _asbp_multiplayer_player_pawn (Utilities|Casting|CastToBP_MultiplayerPlayerPawn Other%20Actor)
      (:then
        (Default|TakeDamage _asbp_multiplayer_player_pawn (Variables|Default|GetDamage)))
      (:CastFailed
        (Utilities|Casting|CastToBP_Projectile Other%20Actor
          (:CastFailed
            _))))
    (CallFunction|MulticastHitEffect Location)
    (CallFunction|ServerEndOfLife)))

(event Custom|EndOfLife
  (CallFunction|ServerEndOfLife))

(event Custom|server_end_of_life
  (Actor|DestroyActor))

(event Custom|server_movement
  (params (DeltaTime :type Float%20%28single-precision%29))
  (Transformation|SetActorLocation (+ (* (Transformation|GetActorForwardVector) (* DeltaTime (Variables|Default|GetSpeed))) (Transformation|GetActorLocation)) false false))

(event Custom|SpawnHitEffect
  (params (Hit%20location :type Vector))
  (Effects|SpawnEmitteratLocation "/Game/StarterContent/Particles/P_Explosion.P_Explosion" Hit%20location))

(event Custom|Multicast%20hit%20effect
  (params (Hit%20location :type Vector))
  (CallFunction|SpawnHitEffect Hit%20location))

(event EventBeginPlay
  (Utilities|Time|SetTimerbyEvent (delegate Custom|EndOfLife) (Variables|Default|GetTTL)))

(event Collision|EventActorBeginOverlap
  (params (OtherActor :type Actor%20Object%20Reference)))

(event EventTick
  (params (DeltaSeconds :type Float%20%28single-precision%29))
  (if (Networking|IsServer)
    (CallFunction|ServerMovement DeltaSeconds)))

(fn ConstructionScript)