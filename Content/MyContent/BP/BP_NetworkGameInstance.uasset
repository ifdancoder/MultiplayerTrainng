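; BP_NetworkGameInstance is a GameInstance Blueprint that handles LAN multiplayer sessions: hosting, listing and joining games.
; CreateGame creates a 16-player session, then opens Lvl1 as a listen server.
; GetGames prints each found session's name, player count and ping, while JoinGame runs its own single-result search and joins that session.
; Session failures and network or travel error events are reported only through PrintString.
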(event Custom|CreateGame
  (|Session (Game|GetPlayerController 0) 16 true
    (:OnSuccess
      (Game|OpenLevel(byName) "Lvl1" true "listen"))
    (:OnFailure
      (Development|PrintString "Start Game error"))))

(event Custom|GetGames
  (bind _results (|FindSessions (Game|GetPlayerController 0) 20 true)
    (:OnSuccess
      (for _array_element _results
        (Development|PrintString (Utilities|String|Append "Server: " (Class|FindSessionsCallbackProxy|GetServerName _array_element) "Players: " (Utilities|String|ToString(Integer) (Class|FindSessionsCallbackProxy|GetCurrentPlayers _array_element)) "/" (Utilities|String|ToString(Integer) (Class|FindSessionsCallbackProxy|GetMaxPlayers _array_element)) "Ping: " (Utilities|String|ToString(Integer) (Class|FindSessionsCallbackProxy|GetPinginMs _array_element))))))
    (:OnFailure
      (Development|PrintString "Failed getting games"))))

(event Custom|Join%20Game
  (bind _returnvalue (Game|GetPlayerController 0))
  (bind _results (|FindSessions _returnvalue 1 true)
    (:OnSuccess
      (for _array_element _results
        (|JoinSession _returnvalue _array_element)))
    (:OnFailure
      (Development|PrintString "Failed joining game"))))

(event EventHandleNetworkError
  (params (FailureType :type ENetworkFailure%20Enum :default "NetDriverAlreadyExists") (bIsServer :type Boolean))
  (Development|PrintString (Utilities|String|Append "Network error: " (Utilities|String|EnumtoString FailureType) "on server: " (Utilities|String|ToString(Boolean) bIsServer))))

(event EventHandleTravelError
  (params (FailureType :type ETravelFailure%20Enum :default "NoLevel"))
  (Development|PrintString (Utilities|String|EnumtoString FailureType)))